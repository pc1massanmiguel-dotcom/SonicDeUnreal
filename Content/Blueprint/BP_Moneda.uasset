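; BP_Moneda is a collectible coin, built as a spinning ring, that BP_Sonic picks up on contact.
; From BeginPlay, a looping short Delay increments the Ring component's relative yaw instead of using Tick, so spin speed depends on frame rate.
; When the Sphere overlaps a BP_Sonic, it increments that character's Monedas counter and destroys itself.
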(event `self.ReceiveBeginPlay`
  (bind _ring (`self.ring`))
  (bind (_relativerotation_roll _relativerotation_pitch _relativerotation_yaw) (`KismetMathLibrary.BreakRotator` (`SceneComponent.RelativeRotation` _ring)))
  (`SceneComponent.K2_SetRelativeRotation` _ring (`KismetMathLibrary.MakeRotator` _relativerotation_roll _relativerotation_pitch (+ _relativerotation_yaw 1.0)) false false :!label _label)
  (`KismetSystemLibrary.Delay` 0.001)
  (goto _label))

(event `self.ReceiveTick`
  (params (DeltaSeconds :type "Float (single-precision)")))

(event `self.Sphere.OnComponentBeginOverlap`
  (params (OverlappedComponent :type "PrimitiveComponent Object Reference") (OtherActor :type "Actor Object Reference") (OtherComp :type "PrimitiveComponent Object Reference") (OtherBodyIndex :type Integer) (bFromSweep :type Boolean) (SweepResult :type "HitResult Structure (by ref)"))
  (bind _asbp_sonic (cast `/Game/Variant_SideScroller/Blueprints/BP_Sonic` OtherActor))
  (set `/Game/Variant_SideScroller/Blueprints/BP_Sonic.Monedas` (+ (`/Game/Variant_SideScroller/Blueprints/BP_Sonic.Monedas` _asbp_sonic) 1) _asbp_sonic)
  (`self.K2_DestroyActor`))

(fn `UserConstructionScript`)