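; BP_Enemigo is a patrolling enemy for a Sonic-style game that can be stomped or hurt the player.
; A looping Delay on BeginPlay nudges it along X, reversing direction and yaw whenever a step counter runs out.
; Sphere overlap destroys it if an undamaged BP_Sonic is falling; otherwise Sonic jumps and briefly loses input.
; A hit opens Lvl_SideScrolling when Sonic has no coins, or zeroes them and spawns one BP_Moneda.
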(event `self.ReceiveBeginPlay`
  (bind (_returnvalue_x _returnvalue_y _returnvalue_z) (`KismetMathLibrary.BreakVector` (`self.K2_GetActorLocation`)))
  (bind _limit (`self.Limit`))
  (bind _defaultsceneroot (`self.DefaultSceneRoot`))
  (`self.K2_SetActorLocation` (`KismetMathLibrary.MakeVector` (+ _returnvalue_x (`self.Valor`)) _returnvalue_y _returnvalue_z) :!label _label)
  (set `self.Limit` (- _limit 1.0))
  (if (== _limit 0.0)
    (if (== (`self.Valor`) -1.0)
      (set `self.Valor` 1.0)
      (`SceneComponent.K2_SetWorldRotation` _defaultsceneroot (struct :`Yaw` -90.0) false false)
      (else
        (set `self.Valor` -1.0)
        (`SceneComponent.K2_SetWorldRotation` _defaultsceneroot (struct :`Yaw` 90.0) false false)))
    (set `self.Limit` 500.0))
  (`KismetSystemLibrary.Delay` 0.01)
  (goto _label))

(event `self.Sphere.OnComponentBeginOverlap`
  (params (OverlappedComponent :type "PrimitiveComponent Object Reference") (OtherActor :type "Actor Object Reference") (OtherComp :type "PrimitiveComponent Object Reference") (OtherBodyIndex :type Integer) (bFromSweep :type Boolean) (SweepResult :type "HitResult Structure (by ref)"))
  (bind _asbp_sonic (cast `/Game/Variant_SideScroller/Blueprints/BP_Sonic` OtherActor))
  (if (and (not (`/Game/Variant_SideScroller/Blueprints/BP_Sonic.Damage` _asbp_sonic)) (`NavMovementComponent.IsFalling` (`Character.CharacterMovement` _asbp_sonic)))
    (`self.K2_DestroyActor`)
    (else
      (`Character.Jump` _asbp_sonic)
      (`self.DisableInput` _asbp_sonic (`GameplayStatics.GetPlayerController` 0))
      (set `/Game/Variant_SideScroller/Blueprints/BP_Sonic.Damage` true _asbp_sonic)
      (if (== (`/Game/Variant_SideScroller/Blueprints/BP_Sonic.Monedas` _asbp_sonic) 0)
        (`KismetSystemLibrary.Delay` 1.0)
        (`GameplayStatics.OpenLevelBySoftObjectPtr` "/Game/Variant_SideScroller/Lvl_SideScrolling.Lvl_SideScrolling")
        (else
          (set `/Game/Variant_SideScroller/Blueprints/BP_Sonic.Monedas` 0 _asbp_sonic)
          (`KismetSystemLibrary.Delay` 1.0)
          (set `/Game/Variant_SideScroller/Blueprints/BP_Sonic.Damage` false _asbp_sonic)
          (`self.EnableInput` _asbp_sonic null)
          (`|SpawnActorFromClass` "/Game/Blueprint/BP_Moneda.BP_Moneda_C" (`KismetMathLibrary.MakeTransform` (`self.K2_GetActorLocation`)) "Undefined" "MultiplyWithRoot" _asbp_sonic null))))))

(fn `UserConstructionScript`)